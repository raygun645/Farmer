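; BP_GridManager builds the farm's soil grid when play begins.
; Nested loops spawn rotated BP_Soil actors on a tile-spaced grid centered on the world origin, spanning the negative to positive row and column counts.
; Tiles on the outer edge get a different crop sprite and a box that blocks all collision channels, forming a border around the field.
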(event `self.ReceiveBeginPlay`
  (bind _gridrows (`self.GridRows`))
  (bind _gridcolumns (`self.GridColumns`))
  (bind _gridrows_2 (`self.GridRows`))
  (bind _gridcolumns_2 (`self.GridColumns`))
  ; creating grid
  (for _index (range (* _gridrows_2 -1) (+ _gridrows_2 1))
    (for _index_2 (range (* _gridcolumns_2 -1) (+ _gridcolumns_2 1))
      (bind _returnvalue (`|SpawnActorFromClass` "/Game/FarmerGameBP/Blueprints/BP_Soil.BP_Soil_C" (`KismetMathLibrary.MakeTransform` (`KismetMathLibrary.MakeVector` (`KismetMathLibrary.Conv_IntToDouble` (* _index (`self.TileSize`))) (`KismetMathLibrary.Conv_IntToDouble` (* _index_2 (`self.TileSize`)))) (struct :`Roll` 90.0)) "Undefined" "MultiplyWithRoot" null null))
      (if (or (== _gridrows _index) (== (* _gridrows -1) _index) (== _gridcolumns _index_2) (== (* _gridcolumns -1) _index_2))
        (`PaperSpriteComponent.SetSprite` (`/Game/FarmerGameBP/Blueprints/BP_Soil.CropSprite` _returnvalue) "/Game/FarmerGameBP/Assets/Sprites/Crops/Tree/Crop_Spritesheet_Plant_Sprite_79.Crop_Spritesheet_Plant_Sprite_79")
        (`PrimitiveComponent.SetCollisionResponseToAllChannels` (`/Game/FarmerGameBP/Blueprints/BP_Soil.Box` _returnvalue) "ECR_Block")))))

(fn `UserConstructionScript`)
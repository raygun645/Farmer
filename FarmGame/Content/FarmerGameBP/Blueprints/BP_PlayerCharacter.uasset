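; Player character for a farming game that moves, hoes, waters and plants on the BP_Soil actors it overlaps.
; Enhanced Input actions send messages to the soil, toggle the crop between turnip and rose, and flip facing through control rotation.
; Successful planting deducts the soil's crop cost, and hoeing pays out when IsCropReady is true after the hoe message.
; BeginPlay adds the mapping context and creates the UI widget showing money.
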(event `EnhancedInput|/Game/FarmerGameBP/Inputs/IA_ChangeCrop`
  (params (ActionValue :type Boolean) (ElapsedSeconds :type "Float (double-precision)") (TriggeredSeconds :type "Float (double-precision)") (InputAction :type "InputAction Object Reference" :default "/Game/FarmerGameBP/Inputs/IA_ChangeCrop.IA_ChangeCrop"))
  (:`Triggered`
    (`/Engine/EditorBlueprintResources/StandardMacros.FlipFlop`
      (:`A`
        (set `self.CurrentCrop` (`self.Turnip`))
        (`KismetSystemLibrary.PrintString` "Crop changed to turnip"))
      (:`B`
        (set `self.CurrentCrop` (`self.Rose`))
        (`KismetSystemLibrary.PrintString` "Crop changed to rose")))))

(event `EnhancedInput|/Game/FarmerGameBP/Inputs/IA_Water`
  (params (ActionValue :type Boolean) (ElapsedSeconds :type "Float (double-precision)") (TriggeredSeconds :type "Float (double-precision)") (InputAction :type "InputAction Object Reference" :default "/Game/FarmerGameBP/Inputs/IA_Water.IA_Water"))
  ; Hoe, Plant and water actions
  (:`Triggered`
    (for _array_element (`self.GetOverlappingActors` "/Game/FarmerGameBP/Blueprints/BP_Soil.BP_Soil_C")
      (message `/Game/FarmerGameBP/Blueprints/BPI_Interaction.Water` _array_element))
    (`GameplayStatics.PlaySound2D` "/Game/FarmerGameBP/Assets/Audio/Water.Water" 1.0 1.0 0.0 null null)))

(event `EnhancedInput|/Game/FarmerGameBP/Inputs/IA_PlantSeed`
  (params (ActionValue :type Boolean) (ElapsedSeconds :type "Float (double-precision)") (TriggeredSeconds :type "Float (double-precision)") (InputAction :type "InputAction Object Reference" :default "/Game/FarmerGameBP/Inputs/IA_PlantSeed.IA_PlantSeed"))
  ; Hoe, Plant and water actions
  (:`Triggered`
    (for _array_element (`self.GetOverlappingActors` "/Game/FarmerGameBP/Blueprints/BP_Soil.BP_Soil_C")
      (bind _cropcost (`/Game/FarmerGameBP/Blueprints/BP_Soil.CropCost` _array_element))
      (if (>= (`self.Money`) _cropcost)
        (bind _wasplanted (message `/Game/FarmerGameBP/Blueprints/BPI_Interaction.Plant` _array_element (`self.CurrentCrop`)))
        (if _wasplanted
          (set `self.Money` (- (`self.Money`) _cropcost))
          (`self.UpdateUI`)
          (`GameplayStatics.PlaySound2D` "/Game/FarmerGameBP/Assets/Audio/Plant.Plant" 1.0 1.0 0.0 null null))))))

(event `EnhancedInput|/Game/FarmerGameBP/Inputs/IA_Hoe`
  (params (ActionValue :type Boolean) (ElapsedSeconds :type "Float (double-precision)") (TriggeredSeconds :type "Float (double-precision)") (InputAction :type "InputAction Object Reference" :default "/Game/FarmerGameBP/Inputs/IA_Hoe.IA_Hoe"))
  ; Hoe, Plant and water actions
  (:`Triggered`
    (`GameplayStatics.PlaySound2D` "/Game/FarmerGameBP/Assets/Audio/Hoe.Hoe" 1.0 1.0 0.0 null null)
    (for _array_element (`self.GetOverlappingActors` "/Game/FarmerGameBP/Blueprints/BP_Soil.BP_Soil_C")
      (`|ExecutionSequence`
        (:`then_0`
          (message `/Game/FarmerGameBP/Blueprints/BPI_Interaction.Hoe` _array_element))
        (:`then_1`
          (if (`/Game/FarmerGameBP/Blueprints/BP_Soil.IsCropReady` _array_element)
            (set `self.Money` (+ (`self.Money`) 20))
            (`self.UpdateUI`)))))))

(event `EnhancedInput|/Game/FarmerGameBP/Inputs/IA_Move`
  (params (ActionValue :type "Vector2D Structure") (ElapsedSeconds :type "Float (double-precision)") (TriggeredSeconds :type "Float (double-precision)") (InputAction :type "InputAction Object Reference" :default "/Game/FarmerGameBP/Inputs/IA_Move.IA_Move"))
  (bind _x (`KismetMathLibrary.BreakVector2D` ActionValue))
  ; Move action
  (:`Triggered`
    (`self.AddMovementInput` (`KismetMathLibrary.Conv_Vector2DToVector` ActionValue))
    (if (!= _x 0.0)
      (`Controller.SetControlRotation` (`self.GetController`) (`KismetMathLibrary.SelectRotator` (`KismetMathLibrary.MakeRotator` 0.0 0.0 180.0) (`KismetMathLibrary.MakeRotator` 0.0) (> _x 0.0))))))

(event `self.ReceiveBeginPlay`
  ; Binding input action + Player UI
  (bind _asplayer_controller (cast `PlayerController` (`self.GetController`)))
  (bind _returnvalue (`|CreateWidget` "/Game/FarmerGameBP/Blueprints/WBP_PlayerUI.WBP_PlayerUI_C" _asplayer_controller))
  (`UserWidget.AddToViewport` _returnvalue 0)
  (`self.UpdateUI`)
  (set `PlayerController.bShowMouseCursor` true _asplayer_controller)
  (message `EnhancedInputSubsystemInterface.AddMappingContext` (pcsubsystem `EnhancedInputLocalPlayerSubsystem` _asplayer_controller) "/Game/FarmerGameBP/Inputs/IMC_FarmerGame.IMC_FarmerGame" 0 (struct))
  (set `self.CurrentCrop` (`self.Rose`)))

(event `UpdateUI`
  ; Money to UI
  (set `TextBlock.Text` (`KismetTextLibrary.Conv_StringToText` (`KismetStringLibrary.Concat_StrStr` "Money - " (`KismetStringLibrary.Conv_IntToString` (`self.Money`)))) (`/Game/FarmerGameBP/Blueprints/WBP_PlayerUI.StatText` (stale `self.ReceiveBeginPlay` _returnvalue))))

(fn `UserConstructionScript`)
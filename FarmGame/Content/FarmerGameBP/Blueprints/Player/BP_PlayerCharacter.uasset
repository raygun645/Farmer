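; Player character for a farming game that moves, picks one of five crops, and hoes, plants, waters and harvests soil.
; Enhanced Input actions set the current crop and value, then send messages to overlapping BP_Soil actors.
; Planting deducts the soil's crop cost when affordable, and hoeing ready crops adds their value to Money.
; BeginPlay creates WBP_PlayerUI, which shows money, the selected crop, toggleable control tips and an animated crop drawer.
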(event `EnhancedInput|/Game/FarmerGameBP/Inputs/IA_ChangeCrop_1`
  (params (ActionValue :type Boolean) (ElapsedSeconds :type "Float (double-precision)") (TriggeredSeconds :type "Float (double-precision)") (InputAction :type "InputAction Object Reference" :default "/Game/FarmerGameBP/Inputs/IA_ChangeCrop_1.IA_ChangeCrop_1"))
  ; Change Crop
  (:`Triggered`
    (set `self.CurrentCrop` (`self.Rose`))
    (set `self.CropValue` (`self.RoseValue`))
    (bind _output_get (set `self.NewCropImage` "/Game/FarmerGameBP/Assets/Sprites/Crops/Rose/Crop_Spritesheet_Plant_Sprite_6.Crop_Spritesheet_Plant_Sprite_6"))
    (`self.UpdateCropImage` _output_get)))

(event `EnhancedInput|/Game/FarmerGameBP/Inputs/IA_ChangeCrop_2`
  (params (ActionValue :type Boolean) (ElapsedSeconds :type "Float (double-precision)") (TriggeredSeconds :type "Float (double-precision)") (InputAction :type "InputAction Object Reference" :default "/Game/FarmerGameBP/Inputs/IA_ChangeCrop_2.IA_ChangeCrop_2"))
  ; Change Crop
  (:`Triggered`
    (set `self.CurrentCrop` (`self.Turnip`))
    (set `self.CropValue` (`self.TurnipValue`))
    (bind _output_get (set `self.NewCropImage` "/Game/FarmerGameBP/Assets/Sprites/Crops/Onion/Crop_Spritesheet_Plant_Sprite_0.Crop_Spritesheet_Plant_Sprite_0"))
    (`self.UpdateCropImage` _output_get)))

(event `EnhancedInput|/Game/FarmerGameBP/Inputs/IA_ChangeCrop_3`
  (params (ActionValue :type Boolean) (ElapsedSeconds :type "Float (double-precision)") (TriggeredSeconds :type "Float (double-precision)") (InputAction :type "InputAction Object Reference" :default "/Game/FarmerGameBP/Inputs/IA_ChangeCrop_3.IA_ChangeCrop_3"))
  ; Change Crop
  (:`Triggered`
    (set `self.CurrentCrop` (`self.Strawberry`))
    (set `self.CropValue` (`self.StrawberryValue`))
    (bind _output_get (set `self.NewCropImage` "/Game/FarmerGameBP/Assets/Sprites/Crops/Strawberry/Crop_Spritesheet_Plant_Sprite_72.Crop_Spritesheet_Plant_Sprite_72"))
    (`self.UpdateCropImage` _output_get)))

(event `EnhancedInput|/Game/FarmerGameBP/Inputs/IA_ChangeCrop_4`
  (params (ActionValue :type Boolean) (ElapsedSeconds :type "Float (double-precision)") (TriggeredSeconds :type "Float (double-precision)") (InputAction :type "InputAction Object Reference" :default "/Game/FarmerGameBP/Inputs/IA_ChangeCrop_4.IA_ChangeCrop_4"))
  ; Change Crop
  (:`Triggered`
    (set `self.CurrentCrop` (`self.Grapes`))
    (set `self.CropValue` (`self.GrapeValue`))
    (bind _output_get (set `self.NewCropImage` "/Game/FarmerGameBP/Assets/Sprites/Crops/Grapes/Crop_Spritesheet_Plant_Sprite_66.Crop_Spritesheet_Plant_Sprite_66"))
    (`self.UpdateCropImage` _output_get)))

(event `EnhancedInput|/Game/FarmerGameBP/Inputs/IA_ChangeCrop_5`
  (params (ActionValue :type Boolean) (ElapsedSeconds :type "Float (double-precision)") (TriggeredSeconds :type "Float (double-precision)") (InputAction :type "InputAction Object Reference" :default "/Game/FarmerGameBP/Inputs/IA_ChangeCrop_5.IA_ChangeCrop_5"))
  ; Change Crop
  (:`Triggered`
    (set `self.CurrentCrop` (`self.Pineapple`))
    (set `self.CropValue` (`self.PineappleValue`))
    (bind _output_get (set `self.NewCropImage` "/Game/FarmerGameBP/Assets/Sprites/Crops/Pineapple/Crop_Spritesheet_Plant_Sprite_48.Crop_Spritesheet_Plant_Sprite_48"))
    (`self.UpdateCropImage` _output_get)))

(event `EnhancedInput|/Game/FarmerGameBP/Inputs/IA_Water`
  (params (ActionValue :type Boolean) (ElapsedSeconds :type "Float (double-precision)") (TriggeredSeconds :type "Float (double-precision)") (InputAction :type "InputAction Object Reference" :default "/Game/FarmerGameBP/Inputs/IA_Water.IA_Water"))
  ; Hoe, Plant and water actions
  (:`Triggered`
    (for _array_element (`self.GetOverlappingActors` "/Game/FarmerGameBP/Blueprints/Level/BP_Soil.BP_Soil_C")
      (message `/Game/FarmerGameBP/Blueprints/Player/BPI_Interaction.Water` _array_element))
    (`GameplayStatics.PlaySound2D` "/Game/FarmerGameBP/Assets/Audio/Water.Water" 1.0 1.0 0.0 null null)))

(event `EnhancedInput|/Game/FarmerGameBP/Inputs/IA_PlantSeed`
  (params (ActionValue :type Boolean) (ElapsedSeconds :type "Float (double-precision)") (TriggeredSeconds :type "Float (double-precision)") (InputAction :type "InputAction Object Reference" :default "/Game/FarmerGameBP/Inputs/IA_PlantSeed.IA_PlantSeed"))
  ; Hoe, Plant and water actions
  (:`Triggered`
    (for _array_element (`self.GetOverlappingActors` "/Game/FarmerGameBP/Blueprints/Level/BP_Soil.BP_Soil_C")
      (bind _cropcost (`/Game/FarmerGameBP/Blueprints/Level/BP_Soil.CropCost` _array_element))
      (if (>= (`self.Money`) _cropcost)
        (bind _wasplanted (message `/Game/FarmerGameBP/Blueprints/Player/BPI_Interaction.Plant` _array_element (`self.CurrentCrop`) (`self.CropValue`)))
        (if _wasplanted
          (set `self.Money` (- (`self.Money`) _cropcost))
          (`self.UpdateMoney`)
          (`GameplayStatics.PlaySound2D` "/Game/FarmerGameBP/Assets/Audio/Plant.Plant" 1.0 1.0 0.0 null null))))))

(event `EnhancedInput|/Game/FarmerGameBP/Inputs/IA_Hoe`
  (params (ActionValue :type Boolean) (ElapsedSeconds :type "Float (double-precision)") (TriggeredSeconds :type "Float (double-precision)") (InputAction :type "InputAction Object Reference" :default "/Game/FarmerGameBP/Inputs/IA_Hoe.IA_Hoe"))
  ; Hoe, Plant and water actions
  (:`Triggered`
    (`GameplayStatics.PlaySound2D` "/Game/FarmerGameBP/Assets/Audio/Hoe.Hoe" 1.0 1.0 0.0 null null)
    (for _array_element (`self.GetOverlappingActors` "/Game/FarmerGameBP/Blueprints/Level/BP_Soil.BP_Soil_C")
      (`|ExecutionSequence`
        (:`then_0`
          (message `/Game/FarmerGameBP/Blueprints/Player/BPI_Interaction.Hoe` _array_element))
        (:`then_1`
          (if (`/Game/FarmerGameBP/Blueprints/Level/BP_Soil.IsCropReady` _array_element)
            (set `self.Money` (+ (`self.Money`) (`/Game/FarmerGameBP/Blueprints/Level/BP_Soil.PlantedCropValue` _array_element)))
            (`self.UpdateMoney`)))))))

(event `EnhancedInput|/Game/FarmerGameBP/Inputs/IA_Move`
  (params (ActionValue :type "Vector2D Structure") (ElapsedSeconds :type "Float (double-precision)") (TriggeredSeconds :type "Float (double-precision)") (InputAction :type "InputAction Object Reference" :default "/Game/FarmerGameBP/Inputs/IA_Move.IA_Move"))
  (bind _x (`KismetMathLibrary.BreakVector2D` ActionValue))
  ; Move action
  (:`Triggered`
    (`self.AddMovementInput` (`KismetMathLibrary.Conv_Vector2DToVector` ActionValue))
    (if (!= _x 0.0)
      (`Controller.SetControlRotation` (`self.GetController`) (`KismetMathLibrary.SelectRotator` (`KismetMathLibrary.MakeRotator` 0.0 0.0 180.0) (`KismetMathLibrary.MakeRotator` 0.0) (> _x 0.0))))))

(event `self.ReceiveBeginPlay`
  ; Binding input action + Player UI
  ;; Set CurrentCrop and irs value
  (set `self.CurrentCrop` (`self.Rose`))
  (set `self.CropValue` (`self.RoseValue`))
  (bind _asplayer_controller (cast `PlayerController` (`self.GetController`)))
  (bind _returnvalue (`|CreateWidget` "/Game/FarmerGameBP/Blueprints/UI/WBP_PlayerUI.WBP_PlayerUI_C" _asplayer_controller))
  (`UserWidget.AddToViewport` _returnvalue 0)
  (`self.UpdateMoney`)
  (set `PlayerController.bShowMouseCursor` true _asplayer_controller)
  (message `EnhancedInputSubsystemInterface.AddMappingContext` (pcsubsystem `EnhancedInputLocalPlayerSubsystem` _asplayer_controller) "/Game/FarmerGameBP/Inputs/IMC_FarmerGame.IMC_FarmerGame" 0 (struct)))

(event `UpdateMoney`
  ; Updating UI
  (set `TextBlock.Text` (`KismetTextLibrary.Conv_StringToText` (`KismetStringLibrary.Concat_StrStr` "$$$ - " (`KismetStringLibrary.Conv_IntToString` (`self.Money`)))) (`/Game/FarmerGameBP/Blueprints/UI/WBP_PlayerUI.MoneyText` (stale `self.ReceiveBeginPlay` _returnvalue))))

(event `UpdateCropImage`
  (params (InBrush :type "PaperSprite Object Reference (by ref)"))
  ; Updating UI
  (`Image.SetBrushResourceObject` (`/Game/FarmerGameBP/Blueprints/UI/WBP_PlayerUI.RoseImage` (stale `self.ReceiveBeginPlay` _returnvalue)) InBrush))

(event `EnhancedInput|/Game/FarmerGameBP/Inputs/IA_TipText`
  (params (ActionValue :type Boolean) (ElapsedSeconds :type "Float (double-precision)") (TriggeredSeconds :type "Float (double-precision)") (InputAction :type "InputAction Object Reference" :default "/Game/FarmerGameBP/Inputs/IA_TipText.IA_TipText"))
  ; Updating UI
  (:`Triggered`
    (`/Engine/EditorBlueprintResources/StandardMacros.FlipFlop`
      (:`A`
        (bind _controlstext (`/Game/FarmerGameBP/Blueprints/UI/WBP_PlayerUI.ControlsText` (stale `self.ReceiveBeginPlay` _returnvalue)))
        (`Widget.SetVisibility` _controlstext "Visible"))
      (:`B`
        (`Widget.SetVisibility` _controlstext "Hidden")))))

(event `EnhancedInput|/Game/FarmerGameBP/Inputs/IA_CropDraw`
  (params (ActionValue :type Boolean) (ElapsedSeconds :type "Float (double-precision)") (TriggeredSeconds :type "Float (double-precision)") (InputAction :type "InputAction Object Reference" :default "/Game/FarmerGameBP/Inputs/IA_CropDraw.IA_CropDraw"))
  ; Updating UI
  (:`Triggered`
    (`/Engine/EditorBlueprintResources/StandardMacros.FlipFlop`
      (:`A`
        (bind _cropdrawanim (`/Game/FarmerGameBP/Blueprints/UI/WBP_PlayerUI.CropDrawAnim` (stale `self.ReceiveBeginPlay` _returnvalue)))
        (`UserWidget.PlayAnimation` (stale `self.ReceiveBeginPlay` _returnvalue) _cropdrawanim 0.0 1 "Forward" 1.0 false))
      (:`B`
        (`UserWidget.PlayAnimation` (stale `self.ReceiveBeginPlay` _returnvalue) _cropdrawanim 0.0 1 "Reverse" 1.0 false)))))

(fn `UserConstructionScript`)
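; Farm soil tile that can be hoed, planted and watered, and grows a crop through sprite stages.
; Hoe, Water and Plant set state flags, soil sprite and crop data; hoeing also clears any crop.
; TimeSkip advances watered crops, dries soil and reverts unplanted ground to unhoed, flagging crops ready at their final stage.
; BeginPlay randomly nudges the crop sprite's position for variation.
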(event `/Game/FarmerGameBP/Blueprints/Player/BPI_Interaction.Hoe`
  ; Hoe Ground
  (`KismetSystemLibrary.DelayUntilNextTick`)
  (`|ExecutionSequence`
    (:`then_0`
      (set `self.SoilIndex` 1)
      (set `self.IsLandHoed` true)
      (set `self.IsWatered` false)
      (set `self.IsCropPlanted` false))
    (:`then_1`
      (`self.UpdateSoilSprite`)
      (`PaperSpriteComponent.SetSprite` (`self.CropSprite`) null))))

(event `self.ReceiveBeginPlay`
  (bind _returnvalue (`KismetMathLibrary.RandomFloatInRange` -5.0 5.0))
  ; Offset for trees
  (`SceneComponent.K2_AddWorldOffset` (`self.CropSprite`) (`KismetMathLibrary.MakeVector` _returnvalue _returnvalue) false false))

(event `/Game/FarmerGameBP/Blueprints/Player/BPI_Interaction.Water`
  ; Water plants
  (if (`self.IsLandHoed`)
    (set `self.SoilIndex` 2)
    (set `self.IsWatered` true)
    (`self.UpdateSoilSprite`)))

(event `/Game/FarmerGameBP/Blueprints/Player/BPI_Interaction.TimeSkip`
  ; TimeSkip
  (`|ExecutionSequence`
    (:`then_0`
      (if (`self.IsCropPlanted`)
        (if (`self.IsWatered`)
          (`/Engine/EditorBlueprintResources/StandardMacros.IncrementInt` (`self.CropIndex`)
            (:`  `
              (set `self.SoilIndex` 1)
              (set `self.IsWatered` false)
              (`self.UpdateCropSprite`))))
        (else
          (set `self.SoilIndex` 0)
          (set `self.IsLandHoed` false))))
    (:`then_1`
      (`self.UpdateSoilSprite`)
      (set `self.IsWatered` false))))

(fn `Plant`
  (params (PlantedSprite :type "Array of PaperSprite Object Reference (by ref)") (ValueOfCrop :type Integer))
  (returns (WasPlanted :type Boolean))
  (if (and (`self.IsLandHoed`) (not (`self.IsCropPlanted`)))
    (set `self.PlantedCropStages` PlantedSprite)
    (set `self.PlantedCropValue` ValueOfCrop)
    (set `self.CropIndex` 0)
    (set `self.IsCropPlanted` true)
    (`self.UpdateCropSprite`)
    (return true)
    (else
      (return false))))

(fn `UpdateCropSprite`
  (bind _plantedcropstages (`self.PlantedCropStages`))
  (bind _returnvalue (- (`KismetArrayLibrary.Array_Length` _plantedcropstages) 1))
  (bind _returnvalue_2 (`KismetMathLibrary.Clamp` (`self.CropIndex`) 0 _returnvalue))
  (`PaperSpriteComponent.SetSprite` (`self.CropSprite`) (`|GetArrayItem` _plantedcropstages _returnvalue_2))
  (if (== _returnvalue_2 _returnvalue)
    (set `self.IsCropReady` true)
    (else
      (set `self.IsCropReady` false))))

(fn `UpdateSoilSprite`
  (`PaperSpriteComponent.SetSprite` (`self.RenderComponent`) (`|GetArrayItem` (`self.SoilSpriteStages`) (`self.SoilIndex`))))

(fn `UserConstructionScript`)